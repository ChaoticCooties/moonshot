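; BP_PlayerCharacter is the player character, driven by two movement input axes.
; The UpDown and LeftRight axes add movement input along the actor's forward and right vectors.
; While either axis is non-zero, Tick rotates only the Cube component toward a world-space direction built from the raw axis values.
; The turn uses a shortest-path rotator lerp scaled by DeltaSeconds and RotationSpeed.
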(event `InputAxis|UpDown`
  (params (AxisValue :type "Float (single-precision)"))
  ;[1 1 1] Movement
  (`self.AddMovementInput` (`self.GetActorForwardVector`) AxisValue))

(event `InputAxis|LeftRight`
  (params (AxisValue :type "Float (single-precision)"))
  ;[1 1 1] Movement
  (`self.AddMovementInput` (`self.GetActorRightVector`) AxisValue))

(event `self.ReceiveTick`
  (params (DeltaSeconds :type "Float (single-precision)"))
  ;[1 1 1] Rotation
  (if (or (!= (`self.GetInputAxisValue`) 0.0) (!= (`self.GetInputAxisValue`) 0.0))
    (set `self.direction` (`KismetMathLibrary.MakeVector` (`self.GetInputAxisValue`) (`self.GetInputAxisValue`)))
    (`SceneComponent.K2_SetWorldRotation` (`self.Cube`) (`KismetMathLibrary.RLerp` (`SceneComponent.K2_GetComponentRotation` (`self.Cube`)) (`KismetMathLibrary.Conv_VectorToRotator` (`self.direction`)) (* DeltaSeconds (`self.rotationSpeed`)) true) false false)))

(fn `UserConstructionScript`)