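; Vodka ingredient Blueprint that accepts one lemon or cranberry ingredient to become a mixable drink.
; Its Pouring event casts the incoming item, then detaches and destroys it, clearing the player's held item.
; The matched ingredient sets its flag, reveals its component on the vodka, enables mixing and selects Lemon Martini or Cape Codder as the result.
; Once either ingredient is added, further pours are ignored.
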(event `self.Pouring`
  (params (`Second Item` :type "Actor Object Reference") (`Player Ref` :type "/Game/Player/BP_PlayerCharacter Object Reference"))
  (if (not (or (`self.hasLemon?`) (`self.hasCranberry?`)))
    (bind _asbp_ingredients_lemon (cast `/Game/Ingredients/BP_Ingredients_Lemon` `Second Item`)
      (:`then`
        (`self.K2_DetachFromActor` _asbp_ingredients_lemon "KeepWorld" "KeepWorld" "KeepWorld")
        (set `/Game/Player/BP_PlayerCharacter.HoldingItem` null `Player Ref`)
        (`self.K2_DestroyActor` _asbp_ingredients_lemon)
        (set `self.hasLemon?` true)
        (set `self.ableToMix` true)
        (set `self.MixedDrink` "/Game/Ingredients/MixedDrink/BP_LemonMartini.BP_LemonMartini_C")
        (`SceneComponent.SetVisibility` (`self.Lemon`) true false))
      (:`CastFailed`
        (bind _asbp_ingredients_cranberry (cast `/Game/Ingredients/BP_Ingredients_Cranberry` `Second Item`))
        (`self.K2_DetachFromActor` _asbp_ingredients_cranberry "KeepWorld" "KeepWorld" "KeepWorld")
        (set `/Game/Player/BP_PlayerCharacter.HoldingItem` null `Player Ref`)
        (`self.K2_DestroyActor` _asbp_ingredients_cranberry)
        (set `self.hasCranberry?` true)
        (set `self.ableToMix` true)
        (set `self.MixedDrink` "/Game/Ingredients/MixedDrink/BP_CapeCodder.BP_CapeCodder_C")
        (`SceneComponent.SetVisibility` (`self.Cranberry`) true false)))))

(fn `UserConstructionScript`
  (`parent.UserConstructionScript`))